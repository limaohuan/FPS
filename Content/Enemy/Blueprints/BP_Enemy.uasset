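; BP_Enemy is an enemy character Blueprint that handles walk speed, damage and death.
; BeginPlay sets the movement component's maximum walk speed.
; OnDamage subtracts damage while Health is above zero; on reaching zero, it clamps Health and plays a falling-back death montage.
; It also sets the IsDead Blackboard key, passing the death state to the AI.
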(event `self.ReceiveBeginPlay`
  (set `CharacterMovementComponent.MaxWalkSpeed` 200.0 (`self.CharacterMovement`)))

(event `self.OnDamage`
  (params (DamageValue :type "Float (single-precision)"))
  ; Event OnDamage
  (if (> (`self.Health`) 0.0)
    (bind _output_get (set `self.Health` (- (`self.Health`) DamageValue)))
    (if (<= _output_get 0.0)
      (set `self.Health` 0.0)
      (`self.PlayAnimMontage` "/Game/Enemy/Model/Animations/Falling_Back_Death_Montage.Falling_Back_Death_Montage")
      (`BlackboardComponent.SetValueAsBool` (`AIBlueprintHelperLibrary.GetBlackboard` null) "IsDead" true))))

(fn `UserConstructionScript`)