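; NPC Blueprint that tracks its distance to the player and performs crouch and salute greeting animations.
; Tick refreshes DistanceToPlayer; Crouching and Greeting play montages and fire finish dispatchers whether completed or interrupted.
; DecreaseEnergy sets a looping timer naming itself, while DecreaseNPCEnergy, which decrements Energy while above zero, is never called here.
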(event `self.ReceiveTick`
  (params (DeltaSeconds :type "Float (single-precision)"))
  (bind _distancetoplayer (`self.UpdateDistanceToPlayer`))
  (set `self.DistanceToPlayer` _distancetoplayer))

(event `Crouching`
  (`|PlayMontage` (`self.Mesh`) "/Game/NPC/Models/Animations/Crouching_Montage.Crouching_Montage"
    (:`OnCompleted`
      _)
    (:`OnInterrupted`
      _))
  (`self.OnFinishCrouch`))

(event `Greeting`
  (`|PlayMontage` (`self.Mesh`) "/Game/NPC/Models/Animations/Salute_Montage.Salute_Montage"
    (:`OnCompleted`
      _)
    (:`OnInterrupted`
      _))
  (`self.OnFinishGreet`))

(event `DecreaseEnergy`
  (`KismetSystemLibrary.K2_SetTimer` null "DecreaseEnergy" 0.1 true))

(fn `DecreaseNPCEnergy`
  (bind _energy (`self.Energy`))
  (if (> _energy 0.0)
    (set `self.Energy` (- _energy 1.0))))

(fn `UpdateDistanceToPlayer`
  (returns (DistanceToPlayer :type "Float (double-precision)"))
  (return (`self.GetDistanceTo` (`GameplayStatics.GetPlayerCharacter` 0))))

(fn `UserConstructionScript`)