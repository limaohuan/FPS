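; BP_Route is an NPC patrol route that serves spline points one at a time as world positions.
; GetSplinePointAsWorldPosition returns the PatrolRoute spline point at the current PointIndex.
; IncrementRoute advances that index until the last point, where it sets IsEnd instead of looping or reversing.
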(event `IncrementRoute`
  (if (== (`self.PointIndex`) (- (`SplineComponent.GetNumberOfSplinePoints` (`self.PatrolRoute`)) 1))
    (set `self.IsEnd` true)
    (else
      (set `self.PointIndex` (+ (`self.PointIndex`) 1)))))

(fn `GetSplinePointAsWorldPosition`
  (returns (WorldLocation :type "Vector Structure"))
  (return (`SplineComponent.GetLocationAtSplinePoint` (`self.PatrolRoute`) (`self.PointIndex`) "World")))

(fn `UserConstructionScript`)