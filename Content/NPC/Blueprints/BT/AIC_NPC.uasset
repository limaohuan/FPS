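; AI controller for NPCs that runs the BT_NPC behavior tree on possession and feeds sight perception into its blackboard.
; Perception updates go to HandleSightSence, which keeps only sight stimuli from the player character and stores that actor in the PlayerCharacterKey blackboard entry.
; The key is written without checking whether the stimulus was successfully sensed, and this controller never clears it.
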(event `self.ReceivePossess`
  (params (PossessedPawn :type "Pawn Object Reference"))
  (`self.RunBehaviorTree` "/Game/NPC/Blueprints/BT/BT_NPC.BT_NPC"))

(event `self.AIPerception.OnTargetPerceptionUpdated`
  (params (Actor :type "Actor Object Reference") (Stimulus :type "AIStimulus Structure"))
  (`self.HandleSightSence` Actor Stimulus))

(fn `HandleSightSence`
  (params (SeenActor :type "Actor Object Reference") (Stimulus :type "AIStimulus Structure"))
  (bind _returnvalue (`AIPerceptionSystem.GetSenseClassForStimulus` Stimulus))
  (if (== _returnvalue "/Script/AIModule.AISense_Sight")
    (if (== (`local.SeenActor`) (`GameplayStatics.GetPlayerCharacter` 0))
      (`BlackboardComponent.SetValueAsObject` (`self.Blackboard`) (`self.PlayerCharacterKey`) (`local.SeenActor`))
      (else
        (return)))
    (else
      (return))))

(fn `UserConstructionScript`)